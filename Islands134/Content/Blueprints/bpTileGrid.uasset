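; Tile grid Blueprint that builds a Width by Height grid of copies of one static mesh.
; The construction script adds a mesh component per cell in nested loops, applying the shared material, a uniform XY scale and a separate vertical scale.
; Spacing comes from the mesh's X bounds on both axes, with padding as a fraction of scaled tile size.
; The event graph holds no active logic.
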(event EventBeginPlay)

(event Collision|EventActorBeginOverlap
  (params (OtherActor :type Actor%20Object%20Reference)))

(event EventTick
  (params (DeltaSeconds :type Float%20%28single-precision%29)))

(fn ConstructionScript
  (bind _scale (Variables|Default|GetScale))
  (bind _scale_2 (Variables|Default|GetScale))
  (bind _scale_3 (Variables|Default|GetScale))
  (bind _mesh (Variables|Default|GetMesh))
  (bind _returnvalue (StaticMesh|GetBounds _mesh))
  ;[1 1 1] Get Tile Side Length
  (LocalVariables|SetTile%20Side%20Length (- (.x (.boxextent _returnvalue)) (.x (.origin _returnvalue))))
  (LocalVariables|SetY%20Offset 0.0)
  (for _index (range 0 (- (Variables|Default|GetHeight) 1))
    (LocalVariables|SetX%20Offset 0.0)
    (for _index_2 (range 0 (- (Variables|Default|GetWidth) 1))
      ;[1 1 1] Add Tile
      (bind _returnvalue_2 (AddComponent|AddStaticMeshComponent false (Math|Transform|MakeTransform (Math|Vector|MakeVector (LocalVariables|GetX%20Offset) (LocalVariables|GetY%20Offset) 0.0) "0, 0, 0" (Math|Vector|MakeVector _scale_3 _scale_3 (Variables|Default|GetVertical%20Scale)))))
      (Components|StaticMesh|SetStaticMesh _returnvalue_2 (Variables|Default|GetMesh))
      (Rendering|Material|SetMaterial _returnvalue_2 0 (Variables|Default|GetMaterial))
      ;[1 1 1] Increase X Offset
      (LocalVariables|SetX%20Offset (+ (LocalVariables|GetX%20Offset) (* (Variables|Default|GetPadding) _scale_2 2.0 (LocalVariables|GetTile%20Side%20Length)) (* _scale_2 2.0 (LocalVariables|GetTile%20Side%20Length)))))
    ;[1 1 1] Increase Y Offset
    (LocalVariables|SetY%20Offset (+ (LocalVariables|GetY%20Offset) (* (Variables|Default|GetPadding) _scale 2.0 (LocalVariables|GetTile%20Side%20Length)) (* _scale 2.0 (LocalVariables|GetTile%20Side%20Length))))))