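; Hex grid Blueprint whose construction script currently places three copies of a hexagon mesh rather than a full grid.
; It derives Diameter and ApothemX2 from the larger and smaller scaled X/Y mesh bounds.
; The copies sit at the origin and at those two distances along X.
; The Width by Height tiling logic, with spacing offsets and alternating yaw, is disconnected and never runs.
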(event EventBeginPlay)

(event Collision|EventActorBeginOverlap
  (params (OtherActor :type Actor%20Object%20Reference)))

(event EventTick
  (params (DeltaSeconds :type Float%20%28single-precision%29)))

(fn ConstructionScript
  (bind _mesh_scale (Variables|Default|GetMesh%20Scale))
  (bind _mesh_scale_2 (Variables|Default|GetMesh%20Scale))
  (bind _mesh (Variables|Default|GetMesh))
  (bind _returnvalue (StaticMesh|GetBounds _mesh))
  (bind _returnvalue_2 (- (.x (.boxextent _returnvalue)) (.x (.origin _returnvalue))))
  (bind _returnvalue_3 (- (.y (.boxextent _returnvalue)) (.y (.origin _returnvalue))))
  (bind _returnvalue_4 (* _mesh_scale _returnvalue_3))
  (bind _returnvalue_5 (* _returnvalue_2 _mesh_scale))
  ;[1 1 1] Get Hexagon Diameter and Apothem
  (LocalVariables|SetDiameter (* (Math|Float|Max(Float) _returnvalue_5 _returnvalue_4) _mesh_scale_2))
  (LocalVariables|SetApothem%20x2 (* _mesh_scale_2 (Math|Float|Min(Float) _returnvalue_5 _returnvalue_4)))
  ;[1 1 1] Add Hexagon Mesh
  (bind _returnvalue_6 (AddComponent|AddStaticMeshComponent false (Math|Transform|MakeTransform (Math|Vector|MakeVector (LocalVariables|GetDiameter) 0.0 0.0) (Math|Rotator|MakeRotator 0.0 0.0 0.0) (Math|Conversions|ToVector(Float) (Variables|Default|GetMesh%20Scale)))))
  (Components|StaticMesh|SetStaticMesh _returnvalue_6 (Variables|Default|GetMesh))
  ;[1 1 1] Add Hexagon Mesh
  (bind _returnvalue_7 (AddComponent|AddStaticMeshComponent false (Math|Transform|MakeTransform (Math|Vector|MakeVector (LocalVariables|GetApothem%20x2) 0.0 0.0) (Math|Rotator|MakeRotator 0.0 0.0 0.0) (Math|Conversions|ToVector(Float) (Variables|Default|GetMesh%20Scale)))))
  (Components|StaticMesh|SetStaticMesh _returnvalue_7 (Variables|Default|GetMesh))
  ;[1 1 1] Add Hexagon Mesh
  (bind _returnvalue_8 (AddComponent|AddStaticMeshComponent false (Math|Transform|MakeTransform (Math|Vector|MakeVector 0.0 0.0 0.0) (Math|Rotator|MakeRotator 0.0 0.0 0.0) (Math|Conversions|ToVector(Float) (Variables|Default|GetMesh%20Scale)))))
  (Components|StaticMesh|SetStaticMesh _returnvalue_8 (Variables|Default|GetMesh)))