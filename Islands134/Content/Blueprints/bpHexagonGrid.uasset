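; Grid actor that lays out a Width by Height honeycomb of a chosen mesh and material, presumably hexagonal tiles.
; The construction script derives an apothem-based spacing from the mesh bounds and horizontal scale, then adds one static mesh component per cell in nested loops.
; Every other column shifts half a cell along Y to interlock, and a separate vertical scale sets tile height.
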(event EventBeginPlay)

(event Collision|EventActorBeginOverlap
  (params (OtherActor :type Actor%20Object%20Reference)))

(event EventTick
  (params (DeltaSeconds :type Float%20%28single-precision%29)))

(fn ConstructionScript
  (bind _mesh (Variables|Default|GetMesh))
  (bind _scale (Variables|Default|GetScale))
  (bind _returnvalue (StaticMesh|GetBounds _mesh))
  ;[1 1 1] Get Apothem
  (LocalVariables|SetApothem (* (Math|Float|Min(Float) (- (.x (.boxextent _returnvalue)) (.x (.origin _returnvalue))) (- (.y (.boxextent _returnvalue)) (.y (.origin _returnvalue)))) 0.5 (Variables|Default|GetScale)))
  (LocalVariables|SetVertical%20Offset 0.0)
  (for _index (range 0 (- (Variables|Default|GetHeight) 1))
    (LocalVariables|SetVertical%20Adjustment 0.0)
    (LocalVariables|SetHorizontal%20Offset 0.0)
    (for _index_2 (range 0 (- (Variables|Default|GetWidth) 1))
      (bind _returnvalue_2 (AddComponent|AddStaticMeshComponent false (Math|Transform|MakeTransform (Math|Vector|MakeVector (LocalVariables|GetHorizontal%20Offset) (+ (LocalVariables|GetVertical%20Offset) (LocalVariables|GetVertical%20Adjustment)) 0.0) "0, 0, 0" (Math|Vector|MakeVector _scale _scale (Variables|Default|GetVertical%20Scale)))))
      (Components|StaticMesh|SetStaticMesh _returnvalue_2 (Variables|Default|GetMesh))
      (Rendering|Material|SetMaterial _returnvalue_2 0 (Variables|Default|GetMaterial))
      (LocalVariables|SetHorizontal%20Offset (+ (* (Math|Float|Sqrt 3.0) (LocalVariables|GetApothem) 2.0) (LocalVariables|GetHorizontal%20Offset)))
      (if (== (LocalVariables|GetVertical%20Adjustment) 0.0)
        (LocalVariables|SetVertical%20Adjustment (* 2.0 (LocalVariables|GetApothem)))
        (else
          (LocalVariables|SetVertical%20Adjustment 0.0))))
    (LocalVariables|SetVertical%20Offset (+ (* 4.0 (LocalVariables|GetApothem)) (LocalVariables|GetVertical%20Offset)))))